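; AI character that moves toward a goal actor and climbs over stalled characters of its own class, letting a crowd pile up.
; A looping timer runs sphere traces ahead and overhead for pawns.
; It climbs by repeated timeline-driven LaunchCharacter pushes when the one ahead is nearly stationary and not climbing.
; A character with another on top stops moving and does not climb, acting as a step.
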(event `self.ReceiveBeginPlay`
  (`KismetSystemLibrary.K2_SetTimerDelegate` (delegate `Tick`) (`self.TraceTime`) true))

(event `Tick`
  (`self.TraceT_CS`)
  (`self.TraceF_CS`))

(event `TraceF_CS`
  (bind (_outhit _is) (`self.CF_TraceF` 30.0 0.0 70.0 15.0))
  (if _is
    (if (`self.IsUnder`)
      (`self.UnClimb_CS`)
      (else
        (bind _asjump_bp (cast `/Game/JumpMap/Jump_BP` (`.HitActor` (`GameplayStatics.BreakHitResult` _outhit)))
          (:`then`
            (if (`self.CF_GetSpeed` _asjump_bp)
              (if (`/Game/JumpMap/Jump_BP.IsClimbing` _asjump_bp)
                (`self.UnClimb_CS` :!label _label)
                (else
                  (`self.Climb_CS`)))
              (else
                (goto _label))))
          (:`CastFailed`
            (goto _label)))))
    (else
      (`self.UnClimb_CS`))))

(event `TraceT_CS`
  (bind (_outhit _is) (`self.CF_TraceT` 1.0 30.0))
  (if _is
    (cast `/Game/JumpMap/Jump_BP` (`.HitActor` (`GameplayStatics.BreakHitResult` _outhit))
      (:`then`
        (set `self.IsUnder` true))
      (:`CastFailed`
        (set `self.IsUnder` false :!label _label_2)))
    (else
      (goto _label_2))))

(event `Climb_CS`
  (set `self.IsClimbing` true)
  (`|ExecutionSequence`
    (:`then_1`
      (`Timeline|Climb_T` :!label _label_3
        (:`Update`
          (`self.LaunchCharacter` (+ (* (`self.GetActorForwardVector`) 55.0) (0.0 0.0 450.0)) true true))))))

(event `UnClimb_CS`
  (set `self.IsClimbing` false)
  (goto _label_3 :!via `Stop`))

(event `self.ReceiveTick`
  (params (DeltaSeconds :type "Float (single-precision)"))
  (if (`self.IsUnder`)
    (`Controller.StopMovement` (`AIBlueprintHelperLibrary.GetAIController` self))
    (else
      (`AIController.MoveToActor` (`AIBlueprintHelperLibrary.GetAIController` self) (`self.NewVar_0`) 100.0 true false false null true))))

(fn `CF_GetSpeed`
  (returns (ReturnValue :type Boolean))
  (return (<= (`KismetMathLibrary.VSize` (`self.GetVelocity`)) 5.0)))

(fn `CF_TraceF`
  (params (`距离` :type "Float (double-precision)") (`Z-` :type "Float (double-precision)") (`Z+` :type "Float (double-precision)") (Radius :type "Float (double-precision)"))
  (returns (OutHit :type "HitResult Structure") (Is :type Boolean))
  (bind _returnvalue (+ (`self.K2_GetActorLocation`) (* (`self.GetActorForwardVector`) `距离`)))
  (bind (_outhit _returnvalue_2) (`KismetSystemLibrary.SphereTraceSingleForObjects` (- _returnvalue (`KismetMathLibrary.MakeVector` 0.0 0.0 `Z-`)) (+ _returnvalue (`KismetMathLibrary.MakeVector` 0.0 0.0 `Z+`)) Radius (`|MakeArray` "ObjectTypeQuery3" :!type "EObjectTypeQuery Enum")))
  (return _outhit _returnvalue_2))

(fn `CF_TraceT`
  (params (`距离` :type "Float (double-precision)") (Radius :type "Float (double-precision)"))
  (returns (OutHit :type "HitResult Structure") (Is :type Boolean))
  (bind _returnvalue (+ (`self.K2_GetActorLocation`) (0.0 0.0 90.0)))
  (bind (_outhit _returnvalue_2) (`KismetSystemLibrary.SphereTraceSingleForObjects` _returnvalue (+ _returnvalue (* (`self.GetActorUpVector`) `距离`)) Radius (`|MakeArray` "ObjectTypeQuery3" :!type "EObjectTypeQuery Enum")))
  (return _outhit _returnvalue_2))

(fn `UserConstructionScript`)