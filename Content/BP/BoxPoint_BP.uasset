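; BoxPoint_BP is a box area actor that supplies random points within its bounds, apparently as destinations for AI movement.
; GetPointCS picks random X/Y offsets inside the scaled Box extent, snaps them to a 35-unit grid, rotates them with the actor and adds its location.
; Both box overlap events are empty; the AImoveto_BP index update and debug point drawing are disconnected.
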(event `self.Box.OnComponentBeginOverlap`
  (params (OverlappedComponent :type "PrimitiveComponent Object Reference") (OtherActor :type "Actor Object Reference") (OtherComp :type "PrimitiveComponent Object Reference") (OtherBodyIndex :type Integer) (bFromSweep :type Boolean) (SweepResult :type "HitResult Structure (by ref)")))

(event `self.Box1.OnComponentBeginOverlap`
  (params (OverlappedComponent :type "PrimitiveComponent Object Reference") (OtherActor :type "Actor Object Reference") (OtherComp :type "PrimitiveComponent Object Reference") (OtherBodyIndex :type Integer) (bFromSweep :type Boolean) (SweepResult :type "HitResult Structure (by ref)")))

(fn `GetPoint_CS`
  (returns (Point :type "Vector Structure"))
  (bind (_returnvalue_x _returnvalue_y) (`KismetMathLibrary.BreakVector` (`BoxComponent.GetScaledBoxExtent` (`self.Box`))))
  (bind _output_get (set `self.NewVar_0` (+ (`self.K2_GetActorLocation`) (`KismetMathLibrary.GreaterGreater_VectorRotator` (`KismetMathLibrary.MakeVector` (* (`.ReturnValue` (`KismetMathLibrary.FMod` (`KismetMathLibrary.RandomFloatInRange` (* _returnvalue_x -1.0) _returnvalue_x) 35.0)) 35.0) (* (`.ReturnValue` (`KismetMathLibrary.FMod` (`KismetMathLibrary.RandomFloatInRange` (* _returnvalue_y -1.0) _returnvalue_y) 35.0)) 35.0)) (`self.K2_GetActorRotation`)))))
  (return _output_get))

(fn `UserConstructionScript`)