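; Test character Blueprint that launches itself along a predicted projectile arc when play begins.
; BeginPlay traces a projectile path from the actor along Arrow1's forward vector and draws it with debug arrows.
; After a zero-length delay, SuggestProjectileVelocityCustomArc derives a velocity from path start to predicted hit, which feeds LaunchCharacter.
; Alternative launch and impulse experiments remain disconnected, and UpdateFly_CS is empty.
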(event `self.ReceiveBeginPlay`
  (bind _returnvalue (`SceneComponent.GetForwardVector` (`self.Arrow1`)))
  (`KismetSystemLibrary.PrintString` (`KismetStringLibrary.Concat_StrStr` (`KismetStringLibrary.Conv_DoubleToString` (`KismetMathLibrary.VSize` _returnvalue)) "+++" (`KismetStringLibrary.Conv_DoubleToString` 0.0)) true true (struct :`G` 0.66 :`B` 1.0 :`A` 1.0) 6.0)
  (bind (_outhit _outpathpositions) (`GameplayStatics.Blueprint_PredictProjectilePath_ByTraceChannel` (`self.K2_GetActorLocation`) (* _returnvalue 588.0) true 10.0 "ECC_WorldStatic" true (`|MakeArray` self :!type "Actor Object Reference") "ForDuration" 10.0 10.0 5.0))
  (bind _output_get (set `self.NewVar_0` _outpathpositions))
  (bind (_array_element _array_index) (`/Game/Main/BP/IF/CS_Macros.ForEachLoop` _outpathpositions)
    (:`LoopBody`
      (`KismetSystemLibrary.DrawDebugArrow` _array_element (`|GetArrayItem` _output_get (`KismetMathLibrary.Clamp` (+ _array_index 1) 0 (`KismetArrayLibrary.Array_LastIndex` _output_get))) 15.0 (struct :`R` 1.0 :`A` 1.0) 100.0 10.0))
    (:`Completed`
      (`KismetSystemLibrary.Delay` 0.0)
      (bind _outlaunchvelocity (`GameplayStatics.SuggestProjectileVelocity_CustomArc` (`|GetArrayItem` (`self.NewVar_0`)) (`.Location` (`GameplayStatics.BreakHitResult` _outhit)) 0.0 0.4))
      (`self.LaunchCharacter` _outlaunchvelocity true true))))

(event `UpdateFly_CS`
  (params (StartPos :type "Vector Structure") (EndPos :type "Vector Structure")))

(fn `UserConstructionScript`)