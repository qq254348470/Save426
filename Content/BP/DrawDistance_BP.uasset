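; DrawDistance_BP is a dimension marker that displays a set distance as a millimetre label between two sphere components.
; The construction script multiplies 距离 (distance) by ten for the text, which 偏移 (offset) positions and 横 (horizontal) rolls.
; It places SphereA and SphereB symmetrically along local X at half the distance, inset slightly.
; Event stubs are disabled, and leftover nodes for moving A/B and line tracing never run.
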(fn `UserConstructionScript`
  (bind `_距离` (`self.距离`))
  (bind _returnvalue (- (/ `_距离` 2.0) 10.0))
  (`SceneComponent.K2_SetRelativeLocation` (`self.TextRender`) (+ (`self.偏移`) (0.0 5.0 0.0)) false false)
  (`SceneComponent.K2_SetRelativeRotation` (`self.TextRender`) (`KismetMathLibrary.MakeRotator` (`KismetMathLibrary.SelectFloat` 0.0 -90.0 (`self.横`)) 0.0 90.0) false false)
  (`TextRenderComponent.K2_SetText` (`self.TextRender`) (`|FormatText` "{a}mm" (* `_距离` 10.0)))
  (`SceneComponent.K2_SetRelativeLocation` (`self.SphereA`) (`KismetMathLibrary.MakeVector` (* _returnvalue -1.0)) false false)
  (`SceneComponent.K2_SetRelativeLocation` (`self.SphereB`) (`KismetMathLibrary.MakeVector` _returnvalue) false false))