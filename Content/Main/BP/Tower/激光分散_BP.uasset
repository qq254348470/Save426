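; Tower Blueprint for a splitting laser (激光分散) that spreads beams among randomly chosen actors inside its AllBox volume.
; A delayed Tick loop re-gathers overlapping actors every half second and resets the particle components.
; It points the Hit particle at a random primary actor, picks further actors without repeats, and filters out invalid ones.
; Pooled particle beams then reactivate, fanning from the primary to each secondary through Start and Target actor parameters.
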(event `self.ReceiveBeginPlay`
  (`self.GetBoxActor_CS` :!label _label))

(event `self.ReceiveTick`
  (params (DeltaSeconds :type "Float (single-precision)"))
  (`KismetSystemLibrary.Delay` 0.5)
  (goto _label))

(event `GetBoxActor_CS`
  (set `self.BoxActor` (`PrimitiveComponent.GetOverlappingActors` (`self.AllBox`) "/Script/Engine.Actor"))
  (for _array_element (`self.ParticleCom`)
    (`ActorComponent.SetActive` _array_element false true))
  (`self.UpdateFX01_CS`))

(event `UpdateFX01_CS`
  (bind _randomactor_new (`self.RandomActor_New`))
  (bind _boxactor (`self.BoxActor`))
  (bind _boxactor_2 (`self.BoxActor`))
  (bind _output_get (set `self.Start` (`|GetArrayItem` _boxactor_2 (`KismetMathLibrary.RandomIntegerInRange` 0 (`KismetArrayLibrary.Array_LastIndex` _boxactor_2)))))
  (`KismetArrayLibrary.Array_RemoveItem` (`self.BoxActor`) _output_get)
  (`FXSystemComponent.SetActorParameter` (`self.Hit`) "Target" _output_get)
  (`KismetArrayLibrary.Array_Clear` (`self.RandomActor`))
  (`KismetArrayLibrary.Array_Add` (`self.RandomActor`) (`self.Start`))
  (while (<= (`KismetArrayLibrary.Array_Length` (`self.RandomActor`)) (`self.Target`))
    (bind _output_get_2 (set `self.Start` (`|GetArrayItem` _boxactor (`KismetMathLibrary.RandomIntegerInRange` 0 (`KismetArrayLibrary.Array_LastIndex` _boxactor)))))
    (`KismetArrayLibrary.Array_Add` (`self.RandomActor`) _output_get_2)
    (`KismetArrayLibrary.Array_RemoveItem` (`self.BoxActor`) _output_get_2))
  (`KismetArrayLibrary.Array_Clear` (`self.RandomActor_New`))
  (for _array_element (`self.RandomActor`)
    (`/Game/Main/BP/134.IsValid` _array_element
      (:`Is Valid`
        (`KismetArrayLibrary.Array_Add` (`self.RandomActor_New`) _array_element))
      (:`Is Not Valid`
        (`KismetSystemLibrary.PrintString` "Hello"))))
  (for (_array_element_2 _array_index) (`self.ParticleCom`)
    (if (< _array_index (`KismetArrayLibrary.Array_LastIndex` _randomactor_new))
      (`ActorComponent.SetActive` _array_element_2 true true)
      (`FXSystemComponent.SetActorParameter` _array_element_2 "Start" (`|GetArrayItem` _randomactor_new))
      (`FXSystemComponent.SetActorParameter` _array_element_2 "Target" (`|GetArrayItem` _randomactor_new (+ _array_index 1))))))

(fn `UserConstructionScript`)