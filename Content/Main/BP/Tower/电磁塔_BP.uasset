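; Electromagnetic tower Blueprint that spins, scales in on spawn, and targets AI_BP actors with particle beams.
; Construction builds a pool of particle components on the mesh socket; a looping cooldown timer aims one at each actor inside Sphere.
; Tick also calls ChangeRateCS on those actors.
; Clear_CS starts a faster loop over Fanweiquan overlaps; hits only drive particles, as the damage call is unwired.
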(event `self.ReceiveTick`
  (params (DeltaSeconds :type "Float (single-precision)"))
  (if (`self.True`)
    (`|ExecutionSequence`
      (:`then_0`
        (`SceneComponent.K2_AddRelativeRotation` (`self.Mesh`) (struct :`Yaw` 3.5) false false))
      (:`then_1`
        (for _array_element (`PrimitiveComponent.GetOverlappingActors` (`self.Sphere`) "/Game/Main/BP/AI/AI_BP.AI_BP_C")
          (bind _asai_bp (cast `/Game/Main/BP/AI/AI_BP` _array_element))
          (`/Game/Main/BP/AI/AI_BP.ChangeRate_CS` _asai_bp false))))))

(event `self.ReceiveBeginPlay`
  (`ActorComponent.SetActive` (`self.0`) true false)
  (`SceneComponent.SetRelativeScale3D` (`self.Mesh`) (0.0 0.0 0.0))
  (`SceneComponent.SetRelativeScale3D` (`self.P_hudun_2`) (0.0 0.0 0.0))
  (`ActorComponent.SetActive` (`self.0`) true false)
  (`KismetSystemLibrary.Delay` 0.5)
  (`self.Init_CS`)
  (`KismetSystemLibrary.Delay` 3.0))

(event `Init_CS`
  ;[1 1 1] 注释
  (bind (_direction `_新建轨道_0`) (`Timeline|时间轴_0` :!via `PlayFromStart`)
    (:`Update`
      (`SceneComponent.SetRelativeScale3D` (`self.Mesh`) (`KismetMathLibrary.Conv_DoubleToVector` (* `_新建轨道_0` (`self.Scale`))))
      (`SceneComponent.SetRelativeScale3D` (`self.P_hudun_2`) (`KismetMathLibrary.Conv_DoubleToVector` (* `_新建轨道_0` 1.0))))
    (:`Finished`
      (set `self.True` true)
      (`KismetSystemLibrary.K2_SetTimerDelegate` (delegate `FindTarget_CS`) (`self.CD`) true))))

(event `FindTarget_CS`
  (bind _overlappingactors (`PrimitiveComponent.GetOverlappingActors` (`self.Sphere`) "/Game/Main/BP/AI/AI_BP.AI_BP_C"))
  (bind _returnvalue (`KismetArrayLibrary.Array_LastIndex` _overlappingactors))
  (`ActorComponent.SetActive` (`self.Hit_Start`) false false)
  (for _array_element (`self.ParticleCom`)
    (`ActorComponent.SetActive` _array_element false false))
  (if (>= _returnvalue 0)
    (`ActorComponent.SetActive` (`self.Hit_Start`) true false)
    (for (_array_element_2 _array_index) (`self.ParticleCom`)
      (if (<= _array_index _returnvalue)
        (`self.Hit_CS` _array_element_2 (`|GetArrayItem` _overlappingactors _array_index))))))

(event `Clear_CS`
  (`KismetSystemLibrary.K2_SetTimerDelegate` (delegate `自定义事件_0`) 0.1 true)
  (set `self.Damage` (100.0 101.0)))

(event `自定义事件_0`
  (for (_array_element _array_index) (`PrimitiveComponent.GetOverlappingActors` (`self.fanweiquan`) "/Game/Main/BP/AI/AI_BP.AI_BP_C")
    (`self.Hit_CS` (`|GetArrayItem` (`self.ParticleCom`) _array_index) _array_element)))

(event `Hit_CS`
  (params (Particle :type "FXSystemComponent Object Reference") (Actor :type "Actor Object Reference"))
  (`FXSystemComponent.SetActorParameter` Particle "Target" Actor)
  (`|ExecutionSequence`
    (:`then_0`
      (`ActorComponent.SetActive` Particle true false))
    (:`then_1`
      (bind _asai_bp (cast `/Game/Main/BP/AI/AI_BP` Actor)))))

(fn `UserConstructionScript`
  (`KismetArrayLibrary.Array_Clear` (`self.ParticleCom`))
  (`SceneComponent.SetRelativeScale3D` (`self.Mesh`) (`KismetMathLibrary.Conv_DoubleToVector` (`self.Scale`)))
  (for _ (range 1 (+ (`self.Max`) 1))
    (bind _returnvalue (`AddComponent|NODE_AddParticleSystemComponent-1` :`bManualAttachment` true :`RelativeTransform` (`KismetMathLibrary.MakeTransform` (0.0 0.0 0.0) (struct) (0.06 0.06 0.06))))
    (`KismetArrayLibrary.Array_Add` (`self.ParticleCom`) _returnvalue)
    (`SceneComponent.K2_AttachToComponent` _returnvalue (`self.Mesh`) "01" "KeepRelative" "KeepRelative" "KeepRelative" true)))