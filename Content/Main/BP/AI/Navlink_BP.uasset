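; Smart nav link that makes an AI Character jump to the link's destination when it reaches the link.
; SmartLinkReached passes the agent's location, destination and JumpDuration to CalculateVelocity, then launches the Character with that velocity.
; CalculateVelocity derives a timed ballistic arc with hardcoded gravity, adjusting vertical speed by an X/Y distance threshold.
; Turn-to-target, actor-moving and suggested-arc launch logic remain unconnected.
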(event `self.ReceiveBeginPlay`)

(event `self.ReceiveSmartLinkReached`
  (params (Agent :type "Actor Object Reference") (Destination :type "Vector Structure (by ref)"))
  (bind _ascharacter (cast `Character` Agent))
  (bind (_returnvalue_roll _returnvalue_pitch _returnvalue_yaw) (`KismetMathLibrary.BreakRotator` (`self.K2_GetActorRotation` _ascharacter)))
  (set `self.NewVar_0` _returnvalue_yaw)
  (`|ExecutionSequence`
    (:`then_0`
      (bind _velocity (`self.CalculateVelocity` (`self.JumpDuration`) Destination (`self.K2_GetActorLocation` _ascharacter)))
      (`Character.LaunchCharacter` _ascharacter _velocity true true))))

(fn `CalculateVelocity`
  (params (InDuration :type "Float (double-precision)") (End :type "Vector Structure") (Start :type "Vector Structure"))
  (returns (Velocity :type "Vector Structure"))
  (bind _induration (`self.InDuration`))
  (bind _returnvalue (- (.x End) (.x Start)))
  (bind _returnvalue_2 (- (.y End) (.y Start)))
  (bind _returnvalue_3 (`KismetMathLibrary.SelectFloat` 50.0 1.0 (>= (`KismetMathLibrary.FMax` _returnvalue _returnvalue_2) 800.0)))
  (set `self.InDuration` InDuration)
  (return (`KismetMathLibrary.MakeVector` (/ _returnvalue _induration) (/ _returnvalue_2 _induration) (/ (- (.z End) (+ (.z Start) (* (`KismetMathLibrary.Square` (`self.InDuration`)) -0.5 982.0) _returnvalue_3)) (/ (`self.InDuration`) _returnvalue_3)))))

(fn `UserConstructionScript`)