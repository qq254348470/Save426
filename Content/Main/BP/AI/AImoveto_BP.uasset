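; AI character blueprint that tracks a route through an array of spline objects and destroys itself past the last one.
; BeginPlay calls InitInfoCS and applies Scale.
; CheckPoint_CS calls UpdateIndexCS within a fixed radius of NewPoint, which advances Index and requests the next point at Distance from that spline.
; Movement toward NewPoint is not in these graphs, and the walk-speed timeline and delay are unconnected.
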(event `self.ReceiveBeginPlay`
  (`|ExecutionSequence`
    (:`then_0`
      (`self.InitInfo_CS`))
    (:`then_1`
      (`self.SetActorScale3D` (`self.Scale`)))))

(event `self.UpdateIndex_CS`
  (bind _aimovetospline (`self.AImoveToSpline`))
  (`KismetSystemLibrary.PrintString` "Hello++=update" true true (struct :`G` 0.66 :`B` 1.0 :`A` 1.0) 5.0)
  (bind _output_get (set `self.Index` (+ (`self.Index`) 1)))
  (if (>= _output_get (`KismetArrayLibrary.Array_Length` _aimovetospline))
    (`self.K2_DestroyActor`)
    (else
      (set `self.NewPoint` (`/Game/Main/BP/SpawnMove/Spline_BP.GetDistancePoint_CF` (`|GetArrayItem` _aimovetospline (`self.Index`)) (`self.Distance`))))))

(event `CheckPoint_CS`
  (if (<= (`KismetMathLibrary.VSize` (- (`self.K2_GetActorLocation`) (`self.NewPoint`))) 150.0)
    (`self.UpdateIndex_CS`)))

(fn `UserConstructionScript`
  (`parent.UserConstructionScript`))