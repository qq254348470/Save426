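; Enemy AI character that follows a spline path with a random skeletal mesh, or as a scaled-up, higher-health boss variant.
; A timeline drives its transform along the path, keeping its spawn offset and changing play rate after a delay.
; Damage updates an HP widget and triggers death by sinking or boss animation.
; It also supports a temporary ice freeze via material swapping and a knockback launch into ragdoll.
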(event `self.ReceiveBeginPlay`
  (`|ExecutionSequence`
    (:`then_0`
      (`self.InitInfo_CS`))
    (:`then_1`
      (`self.BossSetting_CS`))
    (:`then_2`
      (`KismetSystemLibrary.Delay` 0.0)
      (`self.MoveSetting_CS` 0.8) ; 0.8
    )
    (:`then_3`
      (`self.ChangeRate_CS` false))))

(event `InitInfo_CS`
  (bind `_模型` (`self.模型`))
  (`SkinnedMeshComponent.SetSkinnedAssetAndUpdate` (`self.Mesh`) (`|GetArrayItem` `_模型` (`KismetMathLibrary.RandomIntegerInRange` 0 (`KismetArrayLibrary.Array_LastIndex` `_模型`))) true)
  (`self.ChangeM_CF` true) ; 记录初始材质
  (bind _ashp_umg (cast `/Game/Main/BP/AI/HP_UMG` (`WidgetComponent.GetUserWidgetObject` (`self.Widget`))))
  (set `self.HP` _ashp_umg))

(event `BossSetting_CS`
  (bind _mesh (`self.Mesh`))
  (if (`self.Boss`)
    (`SceneComponent.SetRelativeScale3D` (`self.Mesh`) (2.0 2.0 2.0))
    (`SceneComponent.SetVisibility` (`self.Widget`) true false)
    (bind _output_get (set `self.CurrentHP` 300.0))
    (set `self.MaxHP` _output_get)
    (`SkinnedMeshComponent.SetSkinnedAssetAndUpdate` _mesh "/Game/NewScene/SK/腐化士兵/跑步.跑步" true)
    (`SkeletalMeshComponent.PlayAnimation` _mesh "/Game/NewScene/SK/腐化士兵/腐化士兵_走.腐化士兵_走" true)))

(event `MoveSetting_CS`
  (params (Rate :type "Float (double-precision)"))
  (`/Engine/EditorBlueprintResources/StandardMacros.IsValid` (`self.SplinePath`)
    (:`Is Valid`
      (bind _output_get (set `self.Rate` Rate))
      (`TimelineComponent.SetPlayRate` (`self.Timeline_移动`) _output_get)
      (set `self.Offset` (- (`self.K2_GetActorLocation`) (`self.K2_GetActorLocation` (`self.SplinePath`))))
      (bind (_direction `_新建轨道_0`) (`Timeline|Timeline_移动` :!via `PlayFromStart`)
        (:`Update`
          (bind _returnvalue (`/Game/Main/BP/SpawnMove/Spline_BP.Wolrd_CS` (`self.SplinePath`) `_新建轨道_0`))
          (if (not (`self.Die`))
            (`self.K2_SetActorTransform` (`KismetMathLibrary.MakeTransform` (+ (.location _returnvalue) (`self.Offset`)) (`KismetMathLibrary.MakeRotator` 0.0 0.0 (.yaw (.rotation _returnvalue))) (`self.Scale`)))))
        (:`Finished`
          (`self.SetActorHiddenInGame` true))))))

(event `ChangeRate_CS`
  (params (Reset :type Boolean))
  (if Reset
    (bind (_direction _rate) (`Timeline|时间轴_0` :!via `PlayFromStart`)
      (:`Update`
        (set `self.UpdateOffset` (- 1.5 _rate))
        (set `CharacterMovementComponent.MaxWalkSpeed` (- 800.0 (* _rate 200.0)) (`self.CharacterMovement`))))
    (else
      (`KismetSystemLibrary.Delay` 10.0)
      (`|ExecutionSequence`
        (:`then_0`
          (bind (_direction_2 _rate_2) (`Timeline|Timeline_ChangeSpeed` :!via `PlayFromStart`)
            (:`Update`
              (`TimelineComponent.SetPlayRate` (`self.Timeline_移动`) _rate_2))))))))

(event `HitDamage_CS`
  (params (Damage :type "Float (double-precision)"))
  (bind _returnvalue (`self.Damage_CF` Damage))
  (if _returnvalue
    (if (`self.Boss`)
      (`SkeletalMeshComponent.PlayAnimation` (`self.Mesh`) "/Game/NewScene/SK/腐化士兵/挂咯.挂咯" false)
      (`TimelineComponent.Stop` (`self.Timeline_移动`))
      (`self.SetActorEnableCollision` false)
      (`KismetSystemLibrary.Delay` (`KismetMathLibrary.RandomFloatInRange` 2.0 3.0))
      (`self.K2_DestroyActor`)
      (else
        (set `self.Die` true)
        (`self.SetActorEnableCollision` false)
        (`TimelineComponent.Stop` (`self.Timeline_移动`))
        (bind (_direction `_新建轨道_0`) (`Timeline|Timeline_Die` :!via `PlayFromStart`)
          (:`Update`
            (`SceneComponent.K2_SetRelativeLocation` (`self.Mesh`) (`KismetMathLibrary.MakeVector` 0.0 0.0 (`KismetMathLibrary.Lerp` -42.683197 -120.0 `_新建轨道_0`)) false false))
          (:`Finished`
            (`KismetSystemLibrary.Delay` (`KismetMathLibrary.RandomFloatInRange` 3.0 5.0))
            (`self.K2_DestroyActor`)))))))

(event `/Game/Main/BP/IF/CS_Interface.Damage_IF`
  (params (Damage :type "Float (single-precision)"))
  (if (> (`self.CurrentHP`) 0.0)
    (`self.HitDamage_CS` Damage)))

(event `self.ReceiveTick`
  (params (DeltaSeconds :type "Float (single-precision)")))

(event `InRange_CS`
  (params (In :type Boolean))
  (if In
    (`/Engine/EditorBlueprintResources/StandardMacros.DoOnce` false :!label _label
      (:`Completed`
        (for (_ _array_index) (`self.Mesh_M`)
          (`PrimitiveComponent.SetMaterial` (`self.Mesh`) _array_index "/Game/Main/Materials/冰冻/Ice_m_Inst.Ice_m_Inst"))
        (`TimelineComponent.Stop` (`self.Timeline_移动`))
        (set `self.MoveRate_Animation` 0.0)
        (`KismetSystemLibrary.Delay` 2.0)
        (if (not (`self.Die`))
          (`TimelineComponent.Play` (`self.Timeline_移动`))
          (`self.ChangeM_CF` false)
          (set `self.MoveRate_Animation` 1.0)
          (`self.Rest_CS`))))))

(event `Rest_CS`
  (goto _label :!via `Reset`))

(event `UpdateIndex_CS`)

(event `CheckPoint_CS`)

(event `Debuff_Par`
  (bind _debuff (`self.Debuff`))
  (`ActorComponent.SetActive` _debuff true false)
  (`KismetSystemLibrary.Delay` (`KismetMathLibrary.RandomFloatInRange` 0.05 0.1))
  (`ActorComponent.SetActive` _debuff false false))

(event `Hit_Par_CS`
  (`ActorComponent.SetActive` (`self.Hit_Par`) true false))

(event `Fly_CS`
  (params (Point :type "Vector Structure"))
  (bind _mesh (`self.Mesh`))
  (bind (_returnvalue_x _returnvalue_y) (`KismetMathLibrary.BreakVector` (* (`KismetMathLibrary.Normal` (- (`self.K2_GetActorLocation`) Point)) (200.0 200.0 100.0))))
  (if (not (`self.Die`))
    (set `self.Die` true)
    (`GameplayStatics.SpawnEmitterAtLocation` "/Game/Effect/Particles/P_shouji03.P_shouji03" (`self.K2_GetActorLocation`))
    (`TimelineComponent.Stop` (`self.Timeline_移动`))
    (`MovementComponent.StopMovementImmediately` (`self.CharacterMovement`))
    (`self.LaunchCharacter` (`KismetMathLibrary.MakeVector` _returnvalue_x _returnvalue_y 350.0) true true) ; 1000
    (`KismetSystemLibrary.Delay` 0.3)
    (`SkeletalMeshComponent.SetAllBodiesSimulatePhysics` _mesh true)
    (`SkeletalMeshComponent.SetAllBodiesPhysicsBlendWeight` _mesh 1.0 true)
    (`PrimitiveComponent.SetCollisionEnabled` _mesh "QueryAndPhysics")
    (`PrimitiveComponent.SetCollisionEnabled` (`self.CapsuleComponent`) "NoCollision")
    (`KismetSystemLibrary.Delay` (`KismetMathLibrary.RandomFloatInRange` 3.0 5.0))
    (`self.K2_DestroyActor`)))

(fn `ChangeM_CF`
  (params (SaveMaterials :type Boolean))
  (if SaveMaterials
    (`KismetArrayLibrary.Array_Clear` (`self.Mesh_M`))
    (set `self.Mesh_M` (`MeshComponent.GetMaterials` (`self.Mesh`)))
    (else
      (for (_array_element _array_index) (`self.Mesh_M`)
        (`PrimitiveComponent.SetMaterial` (`self.Mesh`) _array_index _array_element)))))

(fn `Damage_CF`
  (params (Damage :type "Float (double-precision)"))
  (returns (ReturnValue :type Boolean))
  (bind _output_get (set `self.CurrentHP` (- (`self.CurrentHP`) Damage)))
  (`/Game/Main/BP/AI/HP_UMG.UpdateHP_CS` (`self.HP`) (/ _output_get (`self.MaxHP`)))
  (return (<= _output_get 0.02)))

(fn `UserConstructionScript`
  (`SkinnedMeshComponent.SetSkinnedAssetAndUpdate` (`self.Mesh`) "/Game/模型资源/3D角色/DD_僵尸类/UE4_通用骨骼/ZombieAB_a.ZombieAB_a" true))