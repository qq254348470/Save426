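; AI actor Blueprint that supplies random roaming destinations around its spawn location.
; BeginPlay calls InitInfoCS, applies the configured scale and stores the start location.
; UpdateIndex_CS picks a navigable NewPoint within a radius of that start and draws a debug point there.
; CheckPoint_CS calls UpdateIndexCS once horizontal distance to NewPoint is within threshold; movement itself is not in this graph.
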(event `self.ReceiveBeginPlay`
  (`|ExecutionSequence`
    (:`then_0`
      (`self.InitInfo_CS`))
    (:`then_1`
      (`self.SetActorScale3D` (`self.Scale`))
      (set `self.StartLocation` (`self.K2_GetActorLocation`)))))

(event `UpdateIndex_CS`
  (bind _randomlocation (`NavigationSystemV1.K2_GetRandomLocationInNavigableRadius` (`self.StartLocation`) 1000.0 null "/Script/NavigationSystem.RecastFilter_UseDefaultArea"))
  (bind _output_get (set `self.NewPoint` _randomlocation))
  (`KismetSystemLibrary.DrawDebugPoint` _output_get 5.0 (struct :`G` 1.0 :`A` 1.0) 10.0))

(event `CheckPoint_CS`
  (bind (_returnvalue_x _returnvalue_y) (`KismetMathLibrary.BreakVector` (- (`self.K2_GetActorLocation`) (`self.NewPoint`))))
  (if (<= (`KismetMathLibrary.VSize` (`KismetMathLibrary.MakeVector` _returnvalue_x _returnvalue_y)) 100.0)
    (`self.UpdateIndex_CS`)))

(fn `UserConstructionScript`
  (`parent.UserConstructionScript`))