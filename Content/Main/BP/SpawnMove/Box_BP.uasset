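; Box volume Blueprint that supplies grid-snapped points within its Box component bounds, spaced by the 间隔XYZ vector.
; GetRandomBoxPointCF returns a random point snapped to that spacing on all three axes around the bounds origin.
; GetAllBoxPointCF rebuilds the Points array as a flat XY grid at the origin's height, returning it with its count.
; The Construction Script draws this grid as yellow debug points; the event graph does nothing at runtime.
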(event `self.ReceiveBeginPlay`)

(fn `GetAllBoxPoint_CF`
  (returns (ReturnValue :type Integer) (`间隔XYZ_0` :type "Array of Vector Structure"))
  (bind (`_间隔xyz_x` `_间隔xyz_y`) (`KismetMathLibrary.BreakVector` (`self.间隔XYZ`)))
  (bind (`_间隔xyz_x_2` `_间隔xyz_y_2`) (`KismetMathLibrary.BreakVector` (`self.间隔XYZ`)))
  (bind _points (`self.Points`))
  (bind (_origin _boxextent) (`KismetSystemLibrary.GetComponentBounds` (`self.Box`)))
  (bind (_remainder _returnvalue) (`KismetMathLibrary.FMod` (.x _boxextent) `_间隔xyz_x_2`))
  (bind (_remainder_2 _returnvalue_2) (`KismetMathLibrary.FMod` (.y _boxextent) `_间隔xyz_y_2`))
  (`KismetArrayLibrary.Array_Clear` (`self.Points`))
  (for _index (range (* _returnvalue -1) (+ _returnvalue 1))
    (for _index_2 (range (* _returnvalue_2 -1) (+ _returnvalue_2 1))
      (`KismetArrayLibrary.Array_Add` (`self.Points`) (+ _origin (`KismetMathLibrary.MakeVector` (* _index `_间隔xyz_x`) (* _index_2 `_间隔xyz_y`))))))
  (return (`KismetArrayLibrary.Array_Length` _points) _points))

(fn `GetRandomBoxPoint_CF`
  (returns (ReturnValue :type "Vector Structure"))
  (bind (`_间隔xyz_x` `_间隔xyz_y` `_间隔xyz_z`) (`KismetMathLibrary.BreakVector` (`self.间隔XYZ`)))
  (bind (`_间隔xyz_x_2` `_间隔xyz_y_2` `_间隔xyz_z_2`) (`KismetMathLibrary.BreakVector` (`self.间隔XYZ`)))
  (bind (_origin _boxextent) (`KismetSystemLibrary.GetComponentBounds` (`self.Box`)))
  (bind _x (.x _boxextent))
  (bind _y (.y _boxextent))
  (bind _z (.z _boxextent))
  (return (+ _origin (`KismetMathLibrary.MakeVector` (* (`.ReturnValue` (`KismetMathLibrary.FMod` (`KismetMathLibrary.RandomFloatInRange` (* _x -1.0) _x) `_间隔xyz_x`)) `_间隔xyz_x_2`) (* (`.ReturnValue` (`KismetMathLibrary.FMod` (`KismetMathLibrary.RandomFloatInRange` (* _y -1.0) _y) `_间隔xyz_y`)) `_间隔xyz_y_2`) (* (`.ReturnValue` (`KismetMathLibrary.FMod` (`KismetMathLibrary.RandomFloatInRange` (* _z -1.0) _z) `_间隔xyz_z`)) `_间隔xyz_z_2`)))))

(fn `UserConstructionScript`
  (bind (_returnvalue `_间隔xyz_0`) (`self.GetAllBoxPoint_CF`))
  (bind _array_element (`/Game/Main/BP/IF/CS_Macros.ForEachLoop` `_间隔xyz_0`)
    (:`LoopBody`
      (`KismetSystemLibrary.DrawDebugPoint` _array_element 10.0 (struct :`R` 1.0 :`G` 1.0 :`A` 1.0) 100.0))))