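; Spawner actor that places wandering AI (AImoveRandom_BP) at random points inside its Box volume.
; BeginPlay (unless Can is set) or StartSpawn_CS arms a non-looping timer for one Spawn, later paused by a delay or End_CS.
; Spawn draws a debug point and passes the Box to the new AI.
; SpawnBossCF separately spawns an enlarged AI_BP in the box's central half, handing it the Spline path and Boss parameter.
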(event `self.ReceiveBeginPlay`
  (if (not (`self.Can`))
    (`KismetSystemLibrary.Delay` 0.0) ; 3
    ;[1 1 1] 生成间隔
    (bind _returnvalue (`KismetSystemLibrary.K2_SetTimerDelegate` (delegate `Spawn`) 0.5 :!label _label)) ; 0.03
    (set `self.Timer` _returnvalue)
    (`KismetSystemLibrary.Delay` 10.0)
    (`KismetSystemLibrary.K2_PauseTimerHandle` (`self.Timer`) :!label _label_2)))

(event `End_CS`
  (goto _label_2))

(event `StartSpawn_CS`
  (goto _label))

(event `Spawn`
  (bind (_returnvalue_x _returnvalue_y) (`KismetMathLibrary.BreakVector` (`BoxComponent.GetScaledBoxExtent` (`self.Box`))))
  (bind _output_get (set `self.NewVar_1` (+ (`KismetMathLibrary.MakeVector` (`KismetMathLibrary.RandomFloatInRange` (* _returnvalue_x -1.0) _returnvalue_x) (`KismetMathLibrary.RandomFloatInRange` (* _returnvalue_y -1.0) _returnvalue_y)) (`self.K2_GetActorLocation`))))
  (`KismetSystemLibrary.DrawDebugPoint` _output_get 5.0 (struct :`R` 1.0 :`A` 1.0) 10.0)
  (`|SpawnActorFromClass` "/Game/Main/BP/AI/AImoveRandom_BP.AImoveRandom_BP_C" (`KismetMathLibrary.MakeTransform` _output_get (struct :`Yaw` -90.0)) "AlwaysSpawn" "OverrideRootScale" null (`self.Box`) null false false (1.0 1.0 1.0) null))

(fn `SpawnBoss_CF`
  (params (Boss :type Boolean))
  (bind (_returnvalue_x _returnvalue_y) (`KismetMathLibrary.BreakVector` (`BoxComponent.GetScaledBoxExtent` (`self.Box`))))
  (`|SpawnActorFromClass` "/Game/Main/BP/AI/AI_BP.AI_BP_C" (`KismetMathLibrary.MakeTransform` (`KismetMathLibrary.MakeVector` (+ (.x (`self.K2_GetActorLocation`)) (`KismetMathLibrary.RandomFloatInRange` (/ (* _returnvalue_x -1.0) 2.0) (/ _returnvalue_x 2.0))) (+ (.y (`self.K2_GetActorLocation`)) (`KismetMathLibrary.RandomFloatInRange` (/ (* _returnvalue_y -1.0) 2.0) (/ _returnvalue_y 2.0))) (.z (`self.K2_GetActorLocation`))) (struct :`Yaw` 90.0) (2.5 2.5 2.5)) "AlwaysSpawn" "OverrideRootScale" null (`self.Spline`) Boss false (1.0 1.0 1.0) null))

(fn `UserConstructionScript`)