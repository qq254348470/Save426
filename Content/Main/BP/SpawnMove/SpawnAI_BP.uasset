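; Spawner actor that feeds spline-following AI into the level and can spawn an enlarged boss AI on request.
; After a BeginPlay delay, a looping timer spawns AImoveto_BP at a random distance point on the first AImoveToSpline, passing along the path references.
; StartSpawn_CS sets the timer again and End_CS pauses it.
; SpawnBossCF places a scaled-up AI_BP randomly within the inner Box area, handing it the Spline and Boss.
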(event `self.ReceiveBeginPlay`
  (`KismetSystemLibrary.Delay` (`self.NewVar_0`)) ; 3
  ;[1 1 1] 生成间隔
  (bind _returnvalue (`KismetSystemLibrary.K2_SetTimerDelegate` (delegate `Spawn`) 0.5 true :!label _label)) ; 0.03
  (set `self.Timer` _returnvalue))

(event `End_CS`
  (`KismetSystemLibrary.K2_PauseTimerHandle` (`self.Timer`)))

(event `StartSpawn_CS`
  (goto _label))

(event `Spawn`
  (bind _output_get (set `self.Distance` (`KismetMathLibrary.RandomFloatInRange` 0.0 1.0)))
  (`|SpawnActorFromClass` "/Game/Main/BP/AI/AImoveto_BP.AImoveto_BP_C" (`KismetMathLibrary.MakeTransform` (`/Game/Main/BP/SpawnMove/Spline_BP.GetDistancePoint_CF` (`|GetArrayItem` (`self.AImoveToSpline`)) _output_get) (struct :`Yaw` -90.0)) "AlwaysSpawn" "OverrideRootScale" null (`self.AImoveToSpline`) (`self.Distance`) 10.0 (`self.Spline`) false false (1.0 1.0 1.0) null))

(fn `SpawnBoss_CF`
  (params (Boss :type Boolean))
  (bind (_returnvalue_x _returnvalue_y) (`KismetMathLibrary.BreakVector` (`BoxComponent.GetScaledBoxExtent` (`self.Box`))))
  (`|SpawnActorFromClass` "/Game/Main/BP/AI/AI_BP.AI_BP_C" (`KismetMathLibrary.MakeTransform` (`KismetMathLibrary.MakeVector` (+ (.x (`self.K2_GetActorLocation`)) (`KismetMathLibrary.RandomFloatInRange` (/ (* _returnvalue_x -1.0) 2.0) (/ _returnvalue_x 2.0))) (+ (.y (`self.K2_GetActorLocation`)) (`KismetMathLibrary.RandomFloatInRange` (/ (* _returnvalue_y -1.0) 2.0) (/ _returnvalue_y 2.0))) (.z (`self.K2_GetActorLocation`))) (struct :`Yaw` 90.0) (2.5 2.5 2.5)) "AlwaysSpawn" "OverrideRootScale" null (`self.Spline`) Boss false (1.0 1.0 1.0) null))

(fn `UserConstructionScript`)