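; Spawner actor that continuously spawns AI_BP characters at random points inside its box area.
; After a startup delay, a fast looping timer fires Spawn, which creates a small batch at random XY offsets within the box extent and passes each the spawner's Spline as its path.
; EndCS pauses the timer to stop spawning.
; The SpawnBoss event is an empty stub, and its timer setup is disconnected.
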(event `EndCS`
  (`KismetSystemLibrary.K2_PauseTimerHandle` (`self.NewVar_3`)))

(event `self.ReceiveBeginPlay`
  ;[1 1 1] 生成间隔
  (`KismetSystemLibrary.Delay` (`self.Delay`))
  (bind _returnvalue (`KismetSystemLibrary.K2_SetTimerDelegate` (delegate `Spawn`) 0.05 true)) ; 0.05
  (set `self.NewVar_3` _returnvalue))

(event `SpawnBoss`)

(event `Spawn`
  (bind (_returnvalue_x _returnvalue_y) (`KismetMathLibrary.BreakVector` (`BoxComponent.GetScaledBoxExtent` (`self.Box`))))
  (for _ (range 2)
    (`|SpawnActorFromClass` "/Game/Main/BP/AI/AI_BP.AI_BP_C" (`KismetMathLibrary.MakeTransform` (`KismetMathLibrary.MakeVector` (+ (.x (`self.K2_GetActorLocation`)) (`KismetMathLibrary.RandomFloatInRange` (* _returnvalue_x -1.0) _returnvalue_x)) (+ (.y (`self.K2_GetActorLocation`)) (`KismetMathLibrary.RandomFloatInRange` (* _returnvalue_y -1.0) _returnvalue_y)) (.z (`self.K2_GetActorLocation`))) (struct :`Yaw` -90.0) (1.3 1.3 1.3)) "AlwaysSpawn" "OverrideRootScale" null (`self.Spline`) false false (1.3 1.3 1.3) null)))

(fn `UserConstructionScript`)